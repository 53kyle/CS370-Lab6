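; Player character with gaze-based interaction and single-button movement, alongside standard axis movement and mouse look.
; Every tick, a 2000-unit Visibility line trace from the camera stores any hit actor implementing BP_interactiveinterface as InteractingActor.
; Pressing moveOrInteract sends that actor an interface message, or, with no valid target, moves the character along the camera's forward vector until released.
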(event Custom|GazeCheck
  (bind _camera (Variables|Default|GetCamera))
  (bind _returnvalue (Transformation|GetWorldLocation _camera))
  (bind _returnvalue_2 (Math|Vector|GetForwardVector _camera))
  ;[1 1 1] Gaze check
  (bind _outhit (Collision|LineTraceByChannel _returnvalue (+ _returnvalue (* _returnvalue_2 2000)) "TraceTypeQuery1" false 0 "ForOneFrame"))
  (if (Utilities|DoesObjectImplementInterface (.HitActor (Collision|BreakHitResult _outhit)) "/Game/Blueprints/BP_interactiveinterface.BP_interactiveinterface_C")
    (Variables|Default|SetinteractingActor (.HitActor (Collision|BreakHitResult _outhit)))
    (else
      (Variables|Default|SetinteractingActor 0)))
  (if (Variables|Default|GetcanMove)
    (bind _output_get (Variables|Default|Setspeed 1e+02))
    (Pawn|Input|AddMovementInput (* _returnvalue_2 (Math|Float|Truncate _output_get)) (Utilities|Time|GetWorldDeltaSeconds) false)))

(event EventTick
  (params (DeltaSeconds :type Float%20%28single-precision%29))
  (CallFunction|GazeCheck))

(event Input|ActionEvents|InputActionmoveOrInteract
  (params (Key :type Key%20Structure :default "None"))
  (bind _interactingactor (Variables|Default|GetinteractingActor))
  ;[1 1 1] Gaze check
  (:Pressed
    (Utilities|IsValid _interactingactor
      (:Is%20Valid
        (Variables|Default|SetcanMove false)
        (Class|BPInteractiveinterface|NewFunction0(Message) _interactingactor))
      (:Is%20Not%20Valid
        (Variables|Default|SetcanMove true))))
  (:Released
    (Variables|Default|SetcanMove false)))

(event Input|AxisEvents|InputAxismouseX
  (params (AxisValue :type Float%20%28single-precision%29))
  ;[1 1 1] Input
  (Pawn|Input|AddControllerYawInput AxisValue))

(event Input|AxisEvents|InputAxismouseY
  (params (AxisValue :type Float%20%28single-precision%29))
  ;[1 1 1] Input
  (Pawn|Input|AddControllerPitchInput AxisValue))

(event Input|AxisEvents|InputAxisMoveLeftRight
  (params (AxisValue :type Float%20%28single-precision%29))
  ;[1 1 1] Input
  (Pawn|Input|AddMovementInput (Transformation|GetActorRightVector) AxisValue false))

(event Input|AxisEvents|InputAxisMoveForwardBack
  (params (AxisValue :type Float%20%28single-precision%29))
  ;[1 1 1] Input
  (Pawn|Input|AddMovementInput (Transformation|GetActorForwardVector) AxisValue false))

(fn ConstructionScript)