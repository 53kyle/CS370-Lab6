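; BP_Light is a light Blueprint whose Sphere switches between glowing and dark through its material.
; On BeginPlay it creates a dynamic material instance from the Sphere's first material slot and stores it as EmissiveMaterial.
; The NewFunction0 event acts as a toggle, flipping IsLit and setting the Emissive vector parameter to white or black.
; Tick and the construction script are empty, and nothing in this graph calls the toggle.
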(event EventBeginPlay
  (bind _returnvalue (Rendering|Material|CreateDynamicMaterialInstance (Variables|Default|GetSphere) 0 (Rendering|Material|GetMaterial (Variables|Default|GetSphere) 0) "None" :!class /Script/Engine.PrimitiveComponent))
  (Variables|Default|SetEmissive%20Material _returnvalue))

(event EventTick
  (params (DeltaSeconds :type Float%20%28single-precision%29)))

(event EventNewFunction0
  (bind _emissive_material (Variables|Default|GetEmissive%20Material))
  (if (Variables|Default|GetisLit)
    (Rendering|Material|SetVectorParameterValue :self _emissive_material :ParameterName "Emissive" :!class /Script/Engine.MaterialInstanceDynamic)
    (Variables|Default|SetisLit false)
    (else
      (Rendering|Material|SetVectorParameterValue _emissive_material "Emissive" "(R=1.000000,G=1.000000,B=1.000000,A=1.000000)" :!class /Script/Engine.MaterialInstanceDynamic)
      (Variables|Default|SetisLit true))))

(fn ConstructionScript)