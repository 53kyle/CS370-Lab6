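; BP_Door is a door actor that slides 200 units up along Z to open and back down to close.
; The NewFunction0 event toggles it by the IsOpen flag, storing the current location before playing Timeline_0 or reversing it to close.
; The timeline's alpha lerps the actor's location without sweep, and IsOpen flips when the timeline finishes.
; Nothing in the blueprint calls the event itself.
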(event EventBeginPlay)

(event Collision|EventActorBeginOverlap
  (params (OtherActor :type Actor%20Object%20Reference)))

(event EventTick
  (params (DeltaSeconds :type Float%20%28single-precision%29)))

(event EventNewFunction0
  (if (Variables|Default|GetisOpen)
    (bind _alpha (Timeline|Timeline_0 Reverse)
      (:Update
        (Transformation|SetActorLocation (Math|Vector|Lerp(Vector) (Variables|Default|GetdoorLocation) (+ (stale _output_get) "0,0,200.000000") _alpha) false false))
      (:Finished
        (if (Variables|Default|GetisOpen)
          (Variables|Default|SetisOpen false)
          (else
            (Variables|Default|SetisOpen true)))))
    (else
      (bind _output_get (Variables|Default|SetdoorLocation (Transformation|GetActorLocation)))
      (Timeline|Timeline_0 Play))))

(fn ConstructionScript)